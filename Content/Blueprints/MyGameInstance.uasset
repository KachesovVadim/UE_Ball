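; Game instance that holds per-level record times and relays UI setup to the HUD.
; SaveRecord and GetRecord switch on the current level name (LVL01 or LVL02), and a record is replaced only by a larger time.
; SetUI lazily caches the GameHUD from player controller 0 and builds the main UI with gun-info and timer visibility flags.
; Init only runs a short delay with nothing after it.
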(event `self.ReceiveInit`
  (`KismetSystemLibrary.Delay` 0.2))

(fn `GetRecord`
  (returns (Record :type "Float (double-precision)"))
  (bind _returnvalue (`GameplayStatics.GetCurrentLevelName` true))
  (switch `string` _returnvalue
    (:`LVL01`
      (return (`self.LVL01Record`)))
    (:`LVL02`
      (return (`self.LVL02Record`)))))

(fn `SaveRecord`
  (params (RecordTime :type "Float (double-precision)"))
  (bind _returnvalue (`GameplayStatics.GetCurrentLevelName` true))
  (switch `string` _returnvalue
    (:`LVL01`
      (if (< (`self.LVL01Record`) RecordTime)
        (set `self.LVL01Record` RecordTime)))
    (:`LVL02`
      (if (< (`self.LVL02Record`) RecordTime)
        (set `self.LVL02Record` RecordTime)))))

(fn `SetUI`
  (params (NeedToShowGunsInfo :type Boolean) (NeedToShowTime :type Boolean))
  (`/Engine/EditorBlueprintResources/StandardMacros.IsValid` (`self.GameHUD`)
    (:`Is Valid`
      _)
    (:`Is Not Valid`
      (bind _output_get (set `self.GameHUD` (cast `/Game/UI/GameHUD` (`PlayerController.GetHUD` (`GameplayStatics.GetPlayerController` 0)) :!pure true)))))
  (`/Game/UI/GameHUD.ConstructMainUI` _output_get NeedToShowGunsInfo NeedToShowTime))