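; Item3 is an interactable item actor that communicates with the UE_BallPawn player through an event dispatcher.
; One second after BeginPlay, it casts the player pawn and binds an event to the pawn's item dispatcher.
; Its interface interact event runs Interact, prints a debug string and calls that dispatcher on the pawn.
; A separate DestroyEvent, apparently the dispatcher's handler, destroys the actor.
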(event `self.ReceiveBeginPlay`
  (`KismetSystemLibrary.Delay` 1.0)
  (add `/Game/Blueprints/UE_BallPawn.ItemDispatcher` (cast `/Game/Blueprints/UE_BallPawn` (`GameplayStatics.GetPlayerPawn` 0) :!pure true) (`|CreateDelegate` :!event `DestroyEvent`)))

(event `/Game/Blueprints/InteractInterface.InteractBPI`
  (`self.Interact`)
  (`KismetSystemLibrary.PrintString` "Item3 interact")
  (`/Game/Blueprints/UE_BallPawn.ItemDispatcher` (cast `/Game/Blueprints/UE_BallPawn` (`GameplayStatics.GetPlayerPawn` 0) :!pure true)))

(event `DestroyEvent`
  (`self.K2_DestroyActor`))

(fn `UserConstructionScript`
  (`parent.UserConstructionScript`))