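; Gun component that manages access to the level's InGameGun actor and forwards primary and secondary shots to it.
; ConstructGuns skips gun setup in LVL01; in other levels it reuses the first existing InGameGun or spawns one at the origin.
; It also returns per-level flags for showing gun info and time, while the shoot calls act only when the gun reference is valid.
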(fn `ConstructGuns`
  (returns (NeedToShowGunsInfo :type Boolean) (NeedToShowTime :type Boolean))
  (bind _returnvalue (`GameplayStatics.GetCurrentLevelName` true))
  (if (`KismetStringLibrary.EqualEqual_StrStr` _returnvalue "LVL01")
    (return false true)
    (else
      (bind _outactors (`GameplayStatics.GetAllActorsOfClass` "/Game/Blueprints/Guns/InGameGun.InGameGun_C"))
      (bind _output (`|GetArrayItem` _outactors))
      (`/Engine/EditorBlueprintResources/StandardMacros.IsValid` _output
        (:`Is Valid`
          (set `self.InGameGun` _output))
        (:`Is Not Valid`
          (bind _returnvalue_2 (`|SpawnActorFromClass` "/Game/Blueprints/Guns/InGameGun.InGameGun_C" (`KismetMathLibrary.MakeTransform` (0.0 0.0 0.0)) "Undefined" "OverrideRootScale" null null))
          (set `self.InGameGun` _returnvalue_2)))
      (bind _returnvalue_3 (`GameplayStatics.GetCurrentLevelName` true))
      (if (`KismetStringLibrary.EqualEqual_StrStr` _returnvalue_3 "LVL03")
        (return true false)
        (else
          (return true true))))))

(fn `GetGun`
  (returns (InGameGun :type "/Game/Blueprints/Guns/InGameGun Object Reference"))
  (return (`self.InGameGun`)))

(fn `ShootFirst`
  (bind _ingamegun (`self.InGameGun`))
  (`/Engine/EditorBlueprintResources/StandardMacros.IsValid` _ingamegun
    (:`Is Valid`
      (`/Game/Blueprints/Guns/InGameGun.ShootFirst` _ingamegun))))

(fn `ShootSecond`
  (bind _ingamegun (`self.InGameGun`))
  (`/Engine/EditorBlueprintResources/StandardMacros.IsValid` _ingamegun
    (:`Is Valid`
      (`/Game/Blueprints/Guns/InGameGun.ShootSecond` _ingamegun))))