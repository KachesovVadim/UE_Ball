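; BasicC is a component that provides shared gameplay actions for what appears to be a physics-driven player actor.
; Interact line-traces from the camera and sends an interface message to the hit actor.
; CompleteGame notifies the GameInstance's HUD and stops physics, SaveRecord passes game time to the GameInstance, and RestartLevel reloads the level.
; DeathFromBall destroys the actor when its combined absolute velocity with an EnemyBall exceeds a threshold.
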(fn `CompleteGame`
  (`/Game/UI/GameHUD.CompleteGame` (`/Game/Blueprints/MyGameInstance.GameHUD` (cast `/Game/Blueprints/MyGameInstance` (`GameplayStatics.GetGameInstance`) :!pure true)))
  (`PrimitiveComponent.SetSimulatePhysics` (`self.PrimitiveComponent`) false))

(fn `DeathFromBall`
  (params (HitActort :type "Actor Object Reference"))
  (bind _asenemy_ball (cast `/Game/Blueprints/Enemies/EnemyBall` HitActort))
  (bind (_returnvalue_x _returnvalue_y _returnvalue_z) (`KismetMathLibrary.BreakVector` (+ (`KismetMathLibrary.Vector_GetAbs` (`SceneComponent.GetComponentVelocity` (`/Game/Blueprints/Enemies/EnemyBall.StaticMesh` _asenemy_ball))) (`KismetMathLibrary.Vector_GetAbs` (`SceneComponent.GetComponentVelocity` (`self.PrimitiveComponent`))))))
  (if (> (+ _returnvalue_x _returnvalue_y _returnvalue_z) 3000.0)
    (`Actor.K2_DestroyActor` (`self.Actor`))))

(fn `Interact`
  (bind _cameracomponent (`self.CameraComponent`))
  (bind _returnvalue (`SceneComponent.K2_GetComponentLocation` _cameracomponent))
  (bind _outhit (`KismetSystemLibrary.LineTraceSingle` _returnvalue (+ _returnvalue (* (`KismetMathLibrary.GetForwardVector` (`SceneComponent.K2_GetComponentRotation` _cameracomponent)) (10000.0 10000.0 10000.0))) "TraceTypeQuery1" true))
  (message `/Game/Blueprints/InteractInterface.InteractBPI` (`.HitActor` (`GameplayStatics.BreakHitResult` _outhit))))

(fn `RestartLevel`
  (bind _returnvalue (`GameplayStatics.GetCurrentLevelName` true))
  (`GameplayStatics.OpenLevel` (`KismetStringLibrary.Conv_StringToName` _returnvalue)))

(fn `SaveRecord`
  (`/Game/Blueprints/MyGameInstance.SaveRecord` (cast `/Game/Blueprints/MyGameInstance` (`GameplayStatics.GetGameInstance`) :!pure true) (`KismetSystemLibrary.GetGameTimeInSeconds`)))