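; ControlC is a movement component that rolls a physics body, likely a ball, by applying force while it is grounded.
; Roll adds a mass-independent force scaled by RollTorque when CanMove is set, which IsOnFloor updates with a short downward line trace from the center of mass.
; UpdateLocation snaps the actor to the primitive's position, and a helper returns values built from negated camera rotation axes.
; Its own BeginPlay and Tick are unused.
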(fn `IsOnFloor`
  (bind _returnvalue (`PrimitiveComponent.GetCenterOfMass` (`self.PrimitiveComponent`) "None"))
  (bind (_outhit _returnvalue_2) (`KismetSystemLibrary.LineTraceSingle` _returnvalue (`KismetMathLibrary.MakeVector` (.x _returnvalue) (.y _returnvalue) (- (.z _returnvalue) 100.0)) "TraceTypeQuery1"))
  (`self.SetCanMove` _returnvalue_2))

(fn `Roll`
  (params (Vector :type "Vector Structure"))
  (if (`self.CanMove`)
    (`PrimitiveComponent.AddForce` (`self.PrimitiveComponent`) (* Vector (`self.RollTorque`)) "None" true)))

(fn `SetCanMove`
  (params (IsCan :type Boolean))
  (set `self.CanMove` IsCan))

(fn `Update View Point Rotation`
  (returns (Rotator :type "Rotator Structure") (Vector :type "Vector Structure"))
  (bind (_x _y _z) (`KismetMathLibrary.BreakRotIntoAxes` (`SceneComponent.K2_GetComponentRotation` (`self.CameraComponent`))))
  (bind _returnvalue (* _y (-1.0 -1.0 -1.0)))
  (return (`KismetMathLibrary.MakeRotationFromAxes` (* _x (-1.0 -1.0 -1.0)) _returnvalue (* _z (-1.0 -1.0 -1.0))) _returnvalue))

(fn `UpdateLocation`
  (`Actor.K2_SetActorLocation` (`self.Actor`) (`SceneComponent.K2_GetComponentLocation` (`self.PrimitiveComponent`)) false false))