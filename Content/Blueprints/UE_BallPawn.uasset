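; Player ball pawn that rolls by camera-relative input, shoots two guns, interacts and handles level completion and restart.
; At BeginPlay it adds three components: ControlC for rolling and floor checks, BasicC for game flow and interaction, GunC for weapons.
; Movement input also repositions the gun above the sphere using the view rotation updated on Tick.
; Destroying the pawn saves the record and restarts the level, so R fades the UI and destroys it.
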(event `self.ReceiveBeginPlay`
  ;[1 1 1] Begin Play
  (bind _returnvalue (`AddComponent|NODE_AddControlC-0` :`PrimitiveComponent` (`self.Sphere`) :`Actor` self :`CameraComponent` (`self.Camera`) :`RollTorque` (`self.RollTorque`)))
  (set `self.ControlC` _returnvalue)
  (bind _returnvalue_2 (`AddComponent|NODE_AddBasicC-0` :`PrimitiveComponent` (`self.Sphere`) :`Actor` self :`CameraComponent` (`self.Camera`)))
  (set `self.BasicC` _returnvalue_2)
  (bind _returnvalue_3 (`AddComponent|NODE_AddGunC-0`))
  (bind _output_get (set `self.GunC` _returnvalue_3))
  (bind (_needtoshowgunsinfo _needtoshowtime) (`/Game/Blueprints/Components/GunC.ConstructGuns` _output_get))
  (`/Game/Blueprints/MyGameInstance.SetUI` (cast `/Game/Blueprints/MyGameInstance` (`GameplayStatics.GetGameInstance`) :!pure true) _needtoshowgunsinfo _needtoshowtime)
  (`KismetSystemLibrary.K2_SetTimer` (`self.ControlC`) "IsOnFloor" 0.5 true)
  (add `self.ItemDispatcher` (`|CreateDelegate` :!event `CompleteGame`)))

(event `InputAxis|MoveRight`
  (params (AxisValue :type "Float (single-precision)"))
  ;[1 1 1] Roll left/right
  (`/Game/Blueprints/Components/ControlC.Roll` (`self.ControlC`) (* AxisValue (`SceneComponent.GetRightVector` (`self.Camera`))))
  (`self.UpdateWeaponsTransform` :!label _label))

(event `InputAxis|MoveForward`
  (params (AxisValue :type "Float (single-precision)"))
  (bind (_returnvalue_x _returnvalue_y) (`KismetMathLibrary.BreakVector` (`SceneComponent.GetForwardVector` (`self.Camera`))))
  ;[1 1 1] Roll forwards/backwards
  (`/Game/Blueprints/Components/ControlC.Roll` (`self.ControlC`) (* AxisValue (`KismetMathLibrary.MakeVector` _returnvalue_x _returnvalue_y)))
  (goto _label))

(event `CompleteGame`
  ;[1 1 1] Complete game
  (`KismetSystemLibrary.Delay` 1.0)
  (`/Game/Blueprints/Components/BasicC.CompleteGame` (`self.BasicC`)))

(event `InputAxis|LookUp`
  (params (AxisValue :type "Float (single-precision)"))
  ;[1 1 1] Turn up-down
  (`self.AddControllerPitchInput` (* AxisValue -1.0)))

(event `InputAxis|Turn`
  (params (AxisValue :type "Float (single-precision)"))
  ;[1 1 1] Turn left-right
  (`self.AddControllerYawInput` AxisValue))

(event `self.ReceiveTick`
  (params (DeltaSeconds :type "Float (single-precision)"))
  (bind _controlc (`self.ControlC`))
  ;[1 1 1] Update pawn location; update weapons rotation; get left gun
  (`/Game/Blueprints/Components/ControlC.UpdateLocation` _controlc)
  (bind (_rotator _vector) (`/Game/Blueprints/Components/ControlC.Update View Point Rotation` _controlc))
  (set `self.ViewPointRotation` _rotator)
  (if (> (.y _vector) 0.0)
    (set `self.LeftGunIsLeft` false)
    (else
      (set `self.LeftGunIsLeft` true))))

(event `self.ReceiveHit`
  (params (MyComp :type "PrimitiveComponent Object Reference") (Other :type "Actor Object Reference") (OtherComp :type "PrimitiveComponent Object Reference") (bSelfMoved :type Boolean) (HitLocation :type "Vector Structure") (HitNormal :type "Vector Structure") (NormalImpulse :type "Vector Structure") (Hit :type "HitResult Structure (by ref)"))
  ;[1 1 1] DeathFromBall
  (`/Game/Blueprints/Components/BasicC.DeathFromBall` (`self.BasicC`) (`.HitActor` (`GameplayStatics.BreakHitResult` Hit))))

(event `Key|E`
  (params (Key :type "Key Structure"))
  ;[1 1 1] InteractSystem
  (:`Pressed`
    (`/Game/Blueprints/Components/BasicC.Interact` (`self.BasicC`))))

(event `Key|LeftMouseButton`
  (params (Key :type "Key Structure"))
  ;[1 1 1] Shoot Mechanic
  (:`Pressed`
    (`/Game/Blueprints/Components/GunC.ShootFirst` (`self.GunC`))))

(event `self.ReceiveDestroyed`
  (bind _basicc (`self.BasicC`))
  ;[1 1 1] Restart game
  (`/Game/Blueprints/Components/BasicC.SaveRecord` _basicc)
  (`/Game/Blueprints/Components/BasicC.RestartLevel` _basicc))

(event `Key|RightMouseButton`
  (params (Key :type "Key Structure"))
  ;[1 1 1] Shoot Mechanic
  (:`Pressed`
    (`/Game/Blueprints/Components/GunC.ShootSecond` (`self.GunC`))))

(event `Key|R`
  (params (Key :type "Key Structure"))
  ;[1 1 1] Restart game
  (:`Pressed`
    (`/Game/UI/MainUI.FadeIn` (`/Game/UI/GameHUD.MainUI` (`/Game/Blueprints/MyGameInstance.GameHUD` (cast `/Game/Blueprints/MyGameInstance` (`GameplayStatics.GetGameInstance`) :!pure true))))
    (`KismetSystemLibrary.Delay` 0.25)
    (`self.K2_DestroyActor`)))

(fn `UpdateWeaponsTransform`
  (bind _ingamegun (`/Game/Blueprints/Components/GunC.GetGun` (`self.GunC`)))
  (bind (_returnvalue_x _returnvalue_y _returnvalue_z) (`KismetMathLibrary.BreakVector` (`PrimitiveComponent.GetCenterOfMass` (`self.Sphere`) "None")))
  (`/Engine/EditorBlueprintResources/StandardMacros.IsValid` _ingamegun
    (:`Is Valid`
      (`/Game/Blueprints/Guns/InGameGun.UpdateTransform` _ingamegun (`KismetMathLibrary.MakeVector` _returnvalue_x _returnvalue_y (+ _returnvalue_z 40.0)) (`self.ViewPointRotation`)))))

(fn `UserConstructionScript`)