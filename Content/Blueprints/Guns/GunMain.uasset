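; Base gun Blueprint providing shared hitscan firing logic through ShootParentFunc, which returns whether the shot fired.
; Each shot line-traces 5000 units from the player camera on the Visibility channel, ignoring the player pawn, and applies multiplied damage to the hit actor.
; It then adds Knockback recoil as pitch and randomized yaw input.
; A timer calling DelayOver re-enables firing after the FireRate interval.
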(fn `DelayOver`
  (set `self.IsDelayOver` true))

(fn `ShootParentFunc`
  (returns (Successful :type Boolean))
  (bind _returnvalue (`GameplayStatics.GetPlayerPawn` 0))
  (bind _returnvalue_2 (`GameplayStatics.GetPlayerCameraManager` 0))
  (bind _knockback (`self.Knockback`))
  (bind _returnvalue_3 (`PlayerCameraManager.GetCameraLocation` _returnvalue_2))
  (if (`self.IsDelayOver`)
    (bind _outhit (`KismetSystemLibrary.LineTraceSingle` _returnvalue_3 (+ _returnvalue_3 (* (`self.GetActorForwardVector` _returnvalue_2) (5000.0 5000.0 5000.0))) "TraceTypeQuery1" false (`|MakeArray` (`GameplayStatics.GetPlayerPawn` 0) :!type "Actor Object Reference")))
    (`GameplayStatics.ApplyDamage` (`.HitActor` (`GameplayStatics.BreakHitResult` _outhit)) (* (`self.DamageMultiplier`) (`self.Damage`)))
    (`Pawn.AddControllerPitchInput` _returnvalue _knockback)
    (`Pawn.AddControllerYawInput` _returnvalue (`KismetMathLibrary.RandomFloatInRange` _knockback (`KismetMathLibrary.Abs` _knockback)))
    (set `self.IsDelayOver` false)
    (`KismetSystemLibrary.K2_SetTimer` null "DelayOver" (`self.FireRate`))
    (return true)
    (else
      (return false))))

(fn `UserConstructionScript`)