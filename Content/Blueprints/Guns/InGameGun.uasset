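; InGameGun is a dual-gun actor holding two Gun1 child actors that rewards alternating fire.
; ShootFirst and ShootSecond fire only when alternated, raising that gun's damage multiplier after each shot, while repeating a side fires nothing and zeroes its multiplier.
; A brief timer gates successive shots.
; UpdateTransform moves the actor and rotates both guns, and GetDamageMultipler exposes each multiplier, treating Gun2 as left.
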(event `ShootFirst`
  (bind _asgun_1 (cast `/Game/Blueprints/Guns/Gun1` (`ChildActorComponent.ChildActor` (`self.Gun1Component`)) :!pure true))
  (if (`self.IsCanShoot`)
    (if (`self.IsFirstGunLastShooted`)
      (set `/Game/Blueprints/Guns/GunMain.DamageMultiplier` 0.0 _asgun_1)
      (else
        (`/Game/Blueprints/Guns/Gun1.ShootChild` _asgun_1)
        (set `self.IsFirstGunLastShooted` true)
        (set `/Game/Blueprints/Guns/GunMain.DamageMultiplier` (+ 0.1 (`/Game/Blueprints/Guns/GunMain.DamageMultiplier` _asgun_1)) _asgun_1)
        (set `self.IsCanShoot` false :!label _label)
        (`KismetSystemLibrary.K2_SetTimer` null "WaitAfterShoot" 0.02)))))

(event `ShootSecond`
  (bind _asgun_1 (cast `/Game/Blueprints/Guns/Gun1` (`ChildActorComponent.ChildActor` (`self.Gun2Component`)) :!pure true))
  (if (`self.IsCanShoot`)
    (if (`self.IsFirstGunLastShooted`)
      (`/Game/Blueprints/Guns/Gun1.ShootChild` _asgun_1)
      (set `self.IsFirstGunLastShooted` false)
      (set `/Game/Blueprints/Guns/GunMain.DamageMultiplier` (+ 0.1 (`/Game/Blueprints/Guns/GunMain.DamageMultiplier` _asgun_1)) _asgun_1)
      (goto _label)
      (else
        (set `/Game/Blueprints/Guns/GunMain.DamageMultiplier` 0.0 _asgun_1)))))

(fn `GetDamageMultipler`
  (params (IsLeftGun :type Boolean))
  (returns (DamageMultiplier :type "Float (double-precision)"))
  (if IsLeftGun
    (bind _asgun_1 (cast `/Game/Blueprints/Guns/Gun1` (`ChildActorComponent.ChildActor` (`self.Gun2Component`)))
      (:`then`
        (return (`/Game/Blueprints/Guns/GunMain.DamageMultiplier` _asgun_1)))
      (:`CastFailed`
        (return 0.0)))
    (else
      (bind _asgun_1_2 (cast `/Game/Blueprints/Guns/Gun1` (`ChildActorComponent.ChildActor` (`self.Gun1Component`)))
        (:`then`
          (return (`/Game/Blueprints/Guns/GunMain.DamageMultiplier` _asgun_1_2)))
        (:`CastFailed`
          (return 0.0))))))

(fn `UpdateTransform`
  (params (Location :type "Vector Structure") (Rotation :type "Rotator Structure"))
  (bind _rotation (`local.Rotation`))
  (`self.K2_SetActorLocation` Location)
  (`SceneComponent.K2_SetRelativeRotation` (`self.Gun1Component`) _rotation false false)
  (`SceneComponent.K2_SetRelativeRotation` (`self.Gun2Component`) _rotation false false))

(fn `UserConstructionScript`)

(fn `WaitAfterShoot`
  (set `self.IsCanShoot` true))