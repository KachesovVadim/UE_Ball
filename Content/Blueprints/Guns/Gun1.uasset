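; Gun1 is a child gun Blueprint that adds recoil animation and a muzzle effect to its parent's shooting logic.
; When the parent's shoot function succeeds, ShootChild kicks the mesh's pitch and spawns the NS_Aura Niagara effect at the Muzzle socket.
; Tick eases the mesh back by a tenth of the remaining angle each frame, so recovery is frame-rate dependent.
; The construction script copies child knockback, fire rate and damage into parent variables.
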(event `ShootChild`
  (bind _successful (`self.ShootParentFunc`))
  (if _successful
    (`SceneComponent.K2_AddLocalRotation` (`self.StaticMesh`) (struct :`Pitch` -30.0) false false)
    (set `self.LeftToTurn` (+ (`self.LeftToTurn`) 30.0))
    (`NiagaraFunctionLibrary.SpawnSystemAttached` "/Game/Parcticles/NS_Aura.NS_Aura" (`self.StaticMesh`) "Muzzle" (0.0 0.0 0.0) (struct :`Pitch` 90.0) "KeepRelativeOffset" true)))

(event `self.ReceiveTick`
  (params (DeltaSeconds :type "Float (single-precision)"))
  (bind _lefttoturn (`self.LeftToTurn`))
  (`SceneComponent.K2_AddLocalRotation` (`self.StaticMesh`) (`KismetMathLibrary.MakeRotator` 0.0 (/ (`self.LeftToTurn`) 10.0)) false false)
  (set `self.LeftToTurn` (- _lefttoturn (/ _lefttoturn 10.0))))

(fn `UserConstructionScript`
  (`parent.UserConstructionScript`)
  (set `self.Knockback` (`self.KnockbackChild`))
  (set `self.FireRate` (`self.FireRateChild`))
  (set `self.Damage` (`self.DamageChild`)))