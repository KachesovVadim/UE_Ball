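; HodakEnemy is an enemy that chases the player's ball pawn and can be killed by damage.
; It spawns its default controller on BeginPlay, then every Tick issues a simple move toward the UE_BallPawn's current location.
; Any damage lowers Health, and a lethal hit spawns a Niagara hit effect at its location and destroys the actor.
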(event `self.ReceiveBeginPlay`
  (`self.SpawnDefaultController`))

(event `self.ReceiveTick`
  (params (DeltaSeconds :type "Float (single-precision)"))
  (bind _asue_ball_pawn (cast `/Game/Blueprints/UE_BallPawn` (`GameplayStatics.GetPlayerPawn` 0)))
  (`AIBlueprintHelperLibrary.SimpleMoveToLocation` (`self.GetController`) (`self.K2_GetActorLocation` _asue_ball_pawn)))

(event `self.ReceiveAnyDamage`
  (params (Damage :type "Float (single-precision)") (DamageType :type "DamageType Object Reference") (InstigatedBy :type "Controller Object Reference") (DamageCauser :type "Actor Object Reference"))
  (bind _returnvalue (- (`self.Health`) Damage))
  (if (> _returnvalue 0.0)
    (set `self.Health` _returnvalue)
    (else
      (`NiagaraFunctionLibrary.SpawnSystemAtLocation` "/Game/Parcticles/NS_BasicHit.NS_BasicHit" (`self.K2_GetActorLocation`))
      (`self.K2_DestroyActor`))))

(fn `UserConstructionScript`)